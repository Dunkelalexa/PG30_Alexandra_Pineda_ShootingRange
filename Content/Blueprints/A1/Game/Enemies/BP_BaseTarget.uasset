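; Base class for shootable targets, flagged as civilian or not, with movement defined by child classes.
; On BeginPlay it calls StartMoving, an empty hook that children override to patrol or slide.
; UpdateMovement lerps the mesh's relative location from its origin to FinalLocation by a given alpha.
; A hit from a BP_ShooterProjectileBase broadcasts OnTargetShot with the civilian flag, then destroys the actor.
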(event EventBeginPlay
  ;[0.15 0.15 0.15 0.5] Each child class overrides StartMoving to define how it moves (patrol or slide)
  (CallFunction|StartMoving))

(event Collision|EventHit
  (params (MyComp :type Primitive%20Component%20Object%20Reference) (Other :type Actor%20Object%20Reference) (OtherComp :type Primitive%20Component%20Object%20Reference) (bSelfMoved :type Boolean) (HitLocation :type Vector :default "0, 0, 0") (HitNormal :type Vector :default "0, 0, 0") (NormalImpulse :type Vector :default "0, 0, 0") (Hit :type Hit%20Result%20Structure%20%28by%20ref%29))
  ;[0.15 0.15 0.15 0.5] notify listeners and destroy the target
  (Utilities|Casting|CastToBP_ShooterProjectileBase Other)
  (CallFunction|HandleShot))

(fn ConstructionScript)

(fn HandleShot
  ;[0.15 0.15 0.15 0.5] let know that was shot (if it was a civil) and destroys after
  (Default|CallOnTargetShot (Variables|Default|GetIsCivilian))
  (Actor|DestroyActor))

(fn UpdateMovement
  (params (Alpha :type Float%20%28double-precision%29))
  ;[0.15 0.15 0.15 0.5] Moves the target to a point between its origin and final location
  (Transformation|SetRelativeLocation (Variables|Default|GetTargetMesh) (Math|Vector|Lerp(Vector) "0, 0, 0" (Variables|Default|Get_FinalLocation) Alpha) false false))

(fn StartMoving
  ;[0.15 0.15 0.15 0.5] Intentionally empty. Child override this to play their own movement
)